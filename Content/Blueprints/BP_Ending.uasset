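; BP_Ending is an overlap trigger that ends the current level with a fade to overexposure and opens the Final level.
; On BeginPlay it caches the first PostProcessVolume found and its original exposure compensation.
; On overlap it disables player pawn input, waits briefly, then plays a timeline that raises exposure compensation.
; The timeline's Update path also runs the delay that precedes the level load.
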(event EventBeginPlay
  (bind _outactors (Actor|GetAllActorsOfClass "/Script/Engine.PostProcessVolume"))
  (bind _output_get (Variables|Default|SetPostProcessRef (Utilities|Array|Get(acopy) _outactors)))
  (Variables|Default|SetOriginalExposureComp (Utilities|Struct|BreakPostProcessSettings (Variables|/Script/Engine.PostProcessVolume|GetSettings _output_get))))

(event Collision|EventActorBeginOverlap
  (params (OtherActor :type Actor%20Object%20Reference))
  (Input|DisableInput (Game|Player|GetPlayerPawn 0) (Game|GetPlayerController 0))
  (Utilities|FlowControl|Delay 1.5)
  (bind _exposurealpha (Timeline|Timeline Play)
    (:Update
      (Utilities|Struct|SetmembersinPostProcessSettings (Variables|/Script/Engine.PostProcessVolume|GetSettings (Variables|Default|GetPostProcessRef)) (Math|Float|Lerp (Variables|Default|GetOriginalExposureComp) 25.0 _exposurealpha))
      (Utilities|FlowControl|Delay 3.0)
      (Game|OpenLevel(byObjectReference) "/Game/Maps/Final.Final"))))

(fn ConstructionScript)